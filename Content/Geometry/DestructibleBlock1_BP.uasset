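; Destructible three-cube wall for the side-scroller that breaks when a dashing character passing the BaseColored crossing check hits it.
; Breaking applies radial damage and explosion effects to each cube, ends the dash, launches the character back and up, plays a sound, then destroys the actor after a delay.
; Tick makes only the first cube query-only while the player dashes.
; The colour material setup is never called.
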(event EventTick
  (params (DeltaSeconds :type Float%20%28single-precision%29))
  (bind _cube_dm (Variables|Default|Getcube_DM))
  ;[1 1 1] Update collision enabled if player is dashing
  (bind _asside_scroller_character (Utilities|Casting|CastToSideScrollerCharacter (Game|GetPlayerCharacter 0)))
  (if (Variables|/Game/SideScrollerCPP/Blueprints/SideScrollerCharacter.SideScrollerCharacter_C|GetbDashing _asside_scroller_character)
    (Collision|SetCollisionEnabled _cube_dm "QueryOnly")
    (else
      (Collision|SetCollisionEnabled _cube_dm "QueryAndPhysics"))))

(event EventBeginPlay
  ;[1 1 1] Init material
)

(event Collision|EventHit
  (params (MyComp :type Primitive%20Component%20Object%20Reference) (Other :type Actor%20Object%20Reference) (OtherComp :type Primitive%20Component%20Object%20Reference) (bSelfMoved :type Boolean) (HitLocation :type Vector :default "0, 0, 0") (HitNormal :type Vector :default "0, 0, 0") (NormalImpulse :type Vector :default "0, 0, 0") (Hit :type Hit%20Result%20Structure%20%28by%20ref%29))
  ;[1 1 1] Destroy on player-dash hit
  (bind _asside_scroller_character (Utilities|Casting|CastToSideScrollerCharacter Other))
  (bind _canbecrossed (Default|CanbeCrossed (Variables|Default|GetBaseColored) _asside_scroller_character))
  (if _canbecrossed
    (if (Variables|/Game/SideScrollerCPP/Blueprints/SideScrollerCharacter.SideScrollerCharacter_C|GetbDashing _asside_scroller_character)
      (CallFunction|DestroyWalls)
      (Variables|/Game/SideScrollerCPP/Blueprints/SideScrollerCharacter.SideScrollerCharacter_C|SetbDashing _asside_scroller_character false)
      (Character|LaunchCharacter _asside_scroller_character (Math|Vector|MakeVector 0.0 (* (.Y (Math|Vector|BreakVector (Transformation|GetActorForwardVector _asside_scroller_character))) -2.5e+03) 2e+03) false true)
      (Audio|SpawnSoundatLocation "/Game/FX/FX_Break_BP.FX_Break_BP" (Transformation|GetActorLocation))
      (Utilities|FlowControl|Delay 5.0)
      (Actor|DestroyActor) ; ToDo - Animación de destrucción
    )))

(fn ConstructionScript)

(fn DisableCollisionwhenPlayerDash
  (params (Object :type Object%20Object%20Reference)))

(fn DisablePhysicswhenPlayerDash
  (params (Object :type Object%20Object%20Reference))
  (bind _cube_dm (Variables|Default|Getcube_DM))
  (bind _asside_scroller_character (Utilities|Casting|CastToSideScrollerCharacter Object)
    (:then
      (if (Variables|/Game/SideScrollerCPP/Blueprints/SideScrollerCharacter.SideScrollerCharacter_C|GetbDashing _asside_scroller_character)
        (Physics|SetSimulatePhysics _cube_dm false)
        (else
          (Physics|SetSimulatePhysics _cube_dm true))))
    (:CastFailed
      (return))))

(fn DestroyWalls
  (bind _returnvalue (Game|GetPlayerCharacter 0))
  (bind _cube_dm3 (Variables|Default|Getcube_DM3))
  (bind _cube_dm (Variables|Default|Getcube_DM))
  (bind _cube_dm2 (Variables|Default|Getcube_DM2))
  (bind _returnvalue_2 (Transformation|GetActorLocation _returnvalue))
  (Utilities|FlowControl|Sequence
    (:then_0
      (Class|DestructibleComponent|ApplyRadiusDamage _cube_dm 1.0 _returnvalue_2 1e+03 5e+03 true)
      (Effects|SpawnEmitteratLocation "/Game/VFX/Particles/Walls/VFX_Wall1_Explosion.VFX_Wall1_Explosion" (Transformation|GetWorldLocation _cube_dm)))
    (:then_1
      (Class|DestructibleComponent|ApplyRadiusDamage _cube_dm2 1.0 _returnvalue_2 1e+03 5e+03 true)
      (Effects|SpawnEmitteratLocation "/Game/VFX/Particles/Walls/VFX_Wall1_Explosion.VFX_Wall1_Explosion" (Transformation|GetWorldLocation _cube_dm2)))
    (:then_2
      (Class|DestructibleComponent|ApplyRadiusDamage _cube_dm3 1.0 _returnvalue_2 1e+03 5e+03 true)
      (Effects|SpawnEmitteratLocation "/Game/VFX/Particles/Walls/VFX_Wall1_Explosion.VFX_Wall1_Explosion" (Transformation|GetWorldLocation _cube_dm3)))))

(fn SetMatearlAllCubes
  (bind _materialinstance (Default|GetMaterialInstance (Variables|Default|GetBaseColored)))
  (Utilities|FlowControl|Sequence
    (:then_0
      (Rendering|Material|SetMaterial (Variables|Default|Getcube_DM) 0 _materialinstance))
    (:then_1
      (Rendering|Material|SetMaterial (Variables|Default|Getcube_DM2) 0 _materialinstance))
    (:then_2
      (Rendering|Material|SetMaterial (Variables|Default|Getcube_DM3) 0 _materialinstance))))