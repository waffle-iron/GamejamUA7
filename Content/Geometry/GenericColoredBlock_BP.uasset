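; GenericColoredBlock is a colored block that the player can pass through when their colors match.
; InitMaterial picks the blue or red material from BlockColor on construction and BeginPlay, and the construction script passes that color to BaseColored with tinting.
; Each tick, BaseColored checks the player character, switching the cube's collision to physics-only when crossable and back to query-and-physics otherwise.
; Unconnected material-tint feedback logic remains unused.
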(event EventTick
  (params (DeltaSeconds :type Float%20%28single-precision%29))
  (bind _cube (Variables|Default|GetCube))
  ;[1 1 1] Update collision enabled if player hasthe same color
  (bind _canbecrossed (Default|CanbeCrossed (Variables|Default|GetBaseColored) (Game|GetPlayerCharacter 0)))
  (if _canbecrossed
    (Collision|SetCollisionEnabled _cube "PhysicsOnly")
    (else
      (Collision|SetCollisionEnabled _cube "QueryAndPhysics"))))

(event EventBeginPlay
  ;[1 1 1] Init - Initial material
  (CallFunction|InitMaterial))

(fn ConstructionScript
  (CallFunction|InitMaterial)
  (Default|SetColor (Variables|Default|GetBaseColored) (Variables|Default|GetBlockColor) true))

(fn InitMaterial
  (bind _cube (Variables|Default|GetCube))
  (switch Utilities|FlowControl|Switch|SwitchonColors_ENUM (Variables|Default|GetBlockColor)
    (:NewEnumerator0
      (Rendering|Material|SetMaterial _cube 0 "/Game/VFX/Materials/NoSolidBlock1_MAT.NoSolidBlock1_MAT"))
    (:NewEnumerator1
      (Rendering|Material|SetMaterial _cube 0 "/Game/VFX/Materials/NoSolidBlock2_MAT.NoSolidBlock2_MAT")))
  (return))