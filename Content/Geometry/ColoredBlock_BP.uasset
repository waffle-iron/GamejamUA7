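; Colored block that lets the player pass through when the player character has a matching color.
; The BaseColored member supplies the color, the material instance and the crossability test for the Cube mesh.
; Each Tick switches Cube collision between PhysicsOnly when crossable and QueryAndPhysics otherwise.
; The material's Color parameter also updates every Tick, turning a dark tint as crossable feedback or restoring the original color.
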(event EventTick
  (params (DeltaSeconds :type Float%20%28single-precision%29))
  (bind _basecolored (Variables|Default|GetBaseColored))
  (bind _basecolored_2 (Variables|Default|GetBaseColored))
  (bind _cube (Variables|Default|GetCube))
  ;[1 1 1] Update collision enabled if player hasthe same color
  (bind _canbecrossed (Default|CanbeCrossed (Variables|Default|GetBaseColored) (Game|GetPlayerCharacter 0)))
  (if _canbecrossed
    (Collision|SetCollisionEnabled _cube "PhysicsOnly")
    ;[1 1 1] Add some feedback for crossed block
    (Default|GetLinearColor _basecolored_2)
    (bind _materialinstance (Default|GetMaterialInstance _basecolored_2))
    (Rendering|Material|SetVectorParameterValue _materialinstance "Color" (Utilities|Struct|MakeLinearColor 0.0 0.0 0.1 0.0) :!class /Script/Engine.MaterialInstanceDynamic)
    (Rendering|Material|SetMaterial (Variables|Default|GetCube) 0 _materialinstance)
    (else
      (Collision|SetCollisionEnabled _cube "QueryAndPhysics")
      ;[1 1 1] Set the original material color
      (bind _newparam (Default|GetLinearColor _basecolored))
      (bind _materialinstance_2 (Default|GetMaterialInstance _basecolored))
      (Rendering|Material|SetVectorParameterValue _materialinstance_2 "Color" _newparam :!class /Script/Engine.MaterialInstanceDynamic)
      (Rendering|Material|SetMaterial (Variables|Default|GetCube) 0 _materialinstance_2))))

(event EventBeginPlay
  ;[1 1 1] Init - Initial material
  (bind _materialinstance (Default|GetMaterialInstance (Variables|Default|GetBaseColored)))
  (Rendering|Material|SetMaterial (Variables|Default|GetCube) 0 _materialinstance))

(fn ConstructionScript)